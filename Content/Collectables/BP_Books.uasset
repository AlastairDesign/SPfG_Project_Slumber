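; BP_Books is a collectable book pickup that bobs up and down.
; When BP_SketchBook_Character overlaps its Box, it adds one to that character's CoinsCollected and destroys itself.
; BeginPlay stores the sprite's starting relative Z, and Tick offsets it with a sine of time since creation, scaled by BobbingSpeed and BobbingDistance.
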(event `self.Box.OnComponentBeginOverlap`
  (params (OverlappedComponent :type "PrimitiveComponent Object Reference") (OtherActor :type "Actor Object Reference") (OtherComp :type "PrimitiveComponent Object Reference") (OtherBodyIndex :type Integer) (bFromSweep :type Boolean) (SweepResult :type "HitResult Structure (by ref)"))
  (bind _asbp_sketch_book_character (cast `/Game/ThirdPerson/Blueprints/BP_SketchBook_Character` OtherActor))
  (set `/Game/ThirdPerson/Blueprints/BP_SketchBook_Character.CoinsCollected` (+ (`/Game/ThirdPerson/Blueprints/BP_SketchBook_Character.CoinsCollected` _asbp_sketch_book_character) 1) _asbp_sketch_book_character)
  (`self.K2_DestroyActor`))

(event `self.ReceiveBeginPlay`
  (set `self.RelativeStaringLocation Z` (.z (.location (`SceneComponent.GetRelativeTransform` (`self.IMG_0395_Sprite`))))))

(event `self.ReceiveTick`
  (params (DeltaSeconds :type "Float (single-precision)"))
  (`SceneComponent.K2_SetRelativeLocation` (`self.IMG_0395_Sprite`) (`KismetMathLibrary.MakeVector` 0.0 0.0 (+ (`self.RelativeStaringLocation Z`) (* (`KismetMathLibrary.DegSin` (* (`self.GetGameTimeSinceCreation`) (`self.BobbingSpeed`))) (`self.BobbingDistance`)))) false false))

(fn `UserConstructionScript`)