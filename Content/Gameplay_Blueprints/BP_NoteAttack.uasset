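; BP_NoteAttack is a note sprite that lights up in colour when the sketchbook player character attacks.
; Every Tick it casts the player character to BP_SketchBook_Character and polls its PencilAttacking and TackAttacking flags.
; When either flag is set, it swaps the PaperSprite to the colour attack note, then restores the black-and-white sprite after a short Delay.
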(event `self.ReceiveTick`
  (params (DeltaSeconds :type "Float (single-precision)"))
  (bind _papersprite (`self.PaperSprite`))
  ; Set colour to attack note
  (bind _asbp_sketch_book_character (cast `/Game/ThirdPerson/Blueprints/BP_SketchBook_Character` (`GameplayStatics.GetPlayerCharacter` 0)))
  (if (`/Game/ThirdPerson/Blueprints/BP_SketchBook_Character.Pencil Attacking` _asbp_sketch_book_character)
    (`PaperSpriteComponent.SetSprite` _papersprite "/Game/Sprites/Notes/attacknote_colour_Sprite.attacknote_colour_Sprite")
    (`KismetSystemLibrary.Delay` 0.5)
    (`PaperSpriteComponent.SetSprite` _papersprite "/Game/Sprites/Notes/attacknote_BW_Sprite.attacknote_BW_Sprite")
    (elif (`/Game/ThirdPerson/Blueprints/BP_SketchBook_Character.Tack Attacking` _asbp_sketch_book_character)
      (`PaperSpriteComponent.SetSprite` _papersprite "/Game/Sprites/Notes/attacknote_colour_Sprite.attacknote_colour_Sprite")
      (`KismetSystemLibrary.Delay` 0.5)
      (`PaperSpriteComponent.SetSprite` _papersprite "/Game/Sprites/Notes/attacknote_BW_Sprite.attacknote_BW_Sprite"))))

(fn `UserConstructionScript`)