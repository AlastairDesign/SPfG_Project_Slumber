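; BP_Sharpener is a consumable pickup that restores the sketchbook character's PencilDamage while the player stands in its box.
; Box overlap events toggle InBox, which Tick checks along with a hardcoded damage threshold, with no input check.
; A Delay on Tick paces each clamped damage increment, which also drains Usage.
; The actor destroys itself once Usage drops below zero.
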(event `self.ReceiveTick`
  (params (DeltaSeconds :type "Float (single-precision)"))
  ; Player Holds E
  (bind _asbp_sketch_book_character (cast `/Game/ThirdPerson/Blueprints/BP_SketchBook_Character` (`GameplayStatics.GetPlayerPawn` 0)))
  ; Will be usable only if pencil damage isn't at max
  (if (`self.InBox`)
    (if (< (`/Game/ThirdPerson/Blueprints/BP_SketchBook_Character.PencilDamage` _asbp_sketch_book_character) 33.0)
      (`KismetSystemLibrary.Delay` 0.4)
      (set `/Game/ThirdPerson/Blueprints/BP_SketchBook_Character.PencilDamage` (`KismetMathLibrary.FClamp` (+ (`/Game/ThirdPerson/Blueprints/BP_SketchBook_Character.PencilDamage` _asbp_sketch_book_character) 1.0) (`/Game/ThirdPerson/Blueprints/BP_SketchBook_Character.MinPencilDamage` _asbp_sketch_book_character) (`/Game/ThirdPerson/Blueprints/BP_SketchBook_Character.MaxPencilDamage` _asbp_sketch_book_character)) _asbp_sketch_book_character)
      ; Using sharpener will degrade sharpener until it is destroyed
      (set `self.Usage` (- (`self.Usage`) 1.0))
      (if (< (`self.Usage`) 0.0)
        (`self.K2_DestroyActor`)))))

(event `self.Box.OnComponentBeginOverlap`
  (params (OverlappedComponent :type "PrimitiveComponent Object Reference") (OtherActor :type "Actor Object Reference") (OtherComp :type "PrimitiveComponent Object Reference") (OtherBodyIndex :type Integer) (bFromSweep :type Boolean) (SweepResult :type "HitResult Structure (by ref)"))
  (cast `/Game/ThirdPerson/Blueprints/BP_SketchBook_Character` OtherActor)
  (set `self.InBox` true))

(event `self.Box.OnComponentEndOverlap`
  (params (OverlappedComponent :type "PrimitiveComponent Object Reference") (OtherActor :type "Actor Object Reference") (OtherComp :type "PrimitiveComponent Object Reference") (OtherBodyIndex :type Integer))
  (cast `/Game/ThirdPerson/Blueprints/BP_SketchBook_Character` OtherActor)
  (set `self.InBox` false))

(fn `UserConstructionScript`)