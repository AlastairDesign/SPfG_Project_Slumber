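; BP_Level_Pad_PC is a level-select pad that loads the Computer_Level when the player interacts while standing on it.
; Box overlap by BP_LevelSelectCharacter creates and shows the WBP_HUD_PC widget, enables input on the actor and opens a gate.
; Leaving the box removes the widget, disables input and closes the gate, which guards the Interact action that triggers the level load.
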(event `InputAction|Interact`
  (params (Key :type "Key Structure"))
  (:`Pressed`
    (`/Engine/EditorBlueprintResources/StandardMacros.Gate` true :!label _label
      (:`Exit`
        (`GameplayStatics.OpenLevelBySoftObjectPtr` "/Game/Level/Computer_Level.Computer_Level")))))

(event `self.Box.OnComponentBeginOverlap`
  (params (OverlappedComponent :type "PrimitiveComponent Object Reference") (OtherActor :type "Actor Object Reference") (OtherComp :type "PrimitiveComponent Object Reference") (OtherBodyIndex :type Integer) (bFromSweep :type Boolean) (SweepResult :type "HitResult Structure (by ref)"))
  (cast `/Game/ThirdPerson/Blueprints/BP_LevelSelectCharacter` OtherActor)
  (bind _returnvalue (`|CreateWidget` "/Game/UI/WBP_HUD_PC.WBP_HUD_PC_C"))
  (bind _output_get (set `self.LevelPadHUDWidget` _returnvalue))
  (`UserWidget.AddToViewport` _output_get 0)
  (`self.EnableInput` (`GameplayStatics.GetPlayerController` 0))
  (goto _label :!via `Open`))

(event `self.Box.OnComponentEndOverlap`
  (params (OverlappedComponent :type "PrimitiveComponent Object Reference") (OtherActor :type "Actor Object Reference") (OtherComp :type "PrimitiveComponent Object Reference") (OtherBodyIndex :type Integer))
  (cast `/Game/ThirdPerson/Blueprints/BP_LevelSelectCharacter` OtherActor)
  (`Widget.RemoveFromParent` (`self.LevelPadHUDWidget`))
  (`self.DisableInput` null)
  (goto _label :!via `Close`))

(fn `UserConstructionScript`)