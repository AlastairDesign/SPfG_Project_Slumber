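; Book-shaped moving platform that bobs its SMBook mesh up and down.
; BeginPlay caches the mesh's starting relative Z as the center of the motion.
; Each Tick sets the relative Z to that base plus a degree-based sine of time since the actor's creation, with BobbingSpeed and BobbingDistance controlling rate and amplitude.
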(event `self.ReceiveBeginPlay`
  (set `self.RelativeStaringLocation Z` (.z (.location (`SceneComponent.GetRelativeTransform` (`self.SM_Book`))))))

(event `self.ReceiveTick`
  (params (DeltaSeconds :type "Float (single-precision)"))
  (`SceneComponent.K2_SetRelativeLocation` (`self.SM_Book`) (`KismetMathLibrary.MakeVector` 0.0 0.0 (+ (`self.RelativeStaringLocation Z`) (* (`KismetMathLibrary.DegSin` (* (`self.GetGameTimeSinceCreation`) (`self.BobbingSpeed`))) (`self.BobbingDistance`)))) false false))

(fn `UserConstructionScript`)